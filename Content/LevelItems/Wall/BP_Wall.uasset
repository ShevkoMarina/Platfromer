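; BP_Wall is a level wall that the player can pass through when the game mode's PassWalls flag is on.
; It caches BP_GameMode on BeginPlay, and each Hit disables the hit component's collision for the player under that flag, otherwise setting it to query and physics.
; A separate BecomePassable function turns off collision for the whole actor.
; Debug prints remain, along with an unconnected overlap-style check that never runs.
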(event `self.ReceiveBeginPlay`
  (bind _asbp_game_mode (cast `/Game/GameMode/BP_GameMode` (`GameplayStatics.GetGameMode`)))
  (set `self.MyGameMode` _asbp_game_mode))

(event `self.ReceiveActorBeginOverlap`
  (params (OtherActor :type "Actor Object Reference")))

(event `self.ReceiveHit`
  (params (MyComp :type "PrimitiveComponent Object Reference") (Other :type "Actor Object Reference") (OtherComp :type "PrimitiveComponent Object Reference") (bSelfMoved :type Boolean) (HitLocation :type "Vector Structure") (HitNormal :type "Vector Structure") (NormalImpulse :type "Vector Structure") (Hit :type "HitResult Structure (by ref)"))
  (bind (_bblockinghit _binitialoverlap _time _distance _location _impactpoint _normal _impactnormal _physmat _hitactor _hitcomponent) (`GameplayStatics.BreakHitResult` Hit))
  ;[1 1 1] Passing though walls
  (if (and (== Other (`GameplayStatics.GetPlayerCharacter` 0)) (`/Game/GameMode/BP_GameMode.PassWalls` (`self.MyGameMode`)))
    (`KismetSystemLibrary.PrintString` "ypu can pass me")
    (`PrimitiveComponent.SetCollisionEnabled` _hitcomponent "NoCollision")
    (else
      (`PrimitiveComponent.SetCollisionEnabled` _hitcomponent "QueryAndPhysics"))))

(fn `BecomePassable`
  (`KismetSystemLibrary.PrintString` "Im passable wall")
  (`self.SetActorEnableCollision` false))

(fn `UserConstructionScript`)