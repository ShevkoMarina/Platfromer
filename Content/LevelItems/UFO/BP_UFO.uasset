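; UFO level hazard that patrols back and forth along X and kills the player on hit by reopening the level.
; ChangeSide chains two two-second MoveComponentTo nodes using MoveForward and MoveBack offsets of MoveDistance, then calls itself to loop.
; The game mode's Deceleration flag selects Stop over Move on each leg; StopForSeconds sets that flag but ignores its time.
; A player hit also sets the game mode's Reload flag.
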(event `self.ReceiveBeginPlay`
  (bind _asbp_game_mode (cast `/Game/GameMode/BP_GameMode` (`GameplayStatics.GetGameMode`)))
  (set `self.MyGameMode` _asbp_game_mode)
  (`self.ChangeSide`))

(event `ChangeSide`
  (bind _defaultsceneroot (`self.DefaultSceneRoot`))
  (bind _defaultsceneroot_2 (`self.DefaultSceneRoot`))
  ;[1 1 1] UFO moving
  (`|ExecutionSequence`
    (:`then_0`
      (bind (_newposition _newrotation) (`self.MoveForward` _defaultsceneroot_2))
      (if (`/Game/GameMode/BP_GameMode.Deceleration` (`self.MyGameMode`))
        (goto _label :!via `Stop`)
        (else
          (`KismetSystemLibrary.MoveComponentTo` _defaultsceneroot_2 _newposition _newrotation false false 2.0 :!label _label)
          (bind (_newposition_2 _newrotation_2) (`self.MoveBack` _defaultsceneroot))
          (if (`/Game/GameMode/BP_GameMode.Deceleration` (`self.MyGameMode`))
            (goto _label_2 :!via `Stop`)
            (else
              (`KismetSystemLibrary.MoveComponentTo` _defaultsceneroot _newposition_2 _newrotation_2 false false 2.0 :!label _label_2)
              (`self.ChangeSide`))))))))

(event `self.ReceiveActorBeginOverlap`
  (params (OtherActor :type "Actor Object Reference"))
  (`KismetSystemLibrary.PrintString` "overplam ufo"))

(event `self.ReceiveHit`
  (params (MyComp :type "PrimitiveComponent Object Reference") (Other :type "Actor Object Reference") (OtherComp :type "PrimitiveComponent Object Reference") (bSelfMoved :type Boolean) (HitLocation :type "Vector Structure") (HitNormal :type "Vector Structure") (NormalImpulse :type "Vector Structure") (Hit :type "HitResult Structure (by ref)"))
  ;[1 1 1] Die when hit
  (if (== Other (`GameplayStatics.GetPlayerCharacter` 0))
    (`KismetSystemLibrary.PrintString` "Ypu died")
    (set `/Game/GameMode/BP_GameMode.Reload` true (`self.MyGameMode`))
    (`GameplayStatics.OpenLevel` "ThirdPersonExampleMap")))

(fn `MoveBack`
  (params (UFO :type "SceneComponent Object Reference"))
  (returns (NewPosition :type "Vector Structure") (NewRotation :type "Rotator Structure"))
  (bind (_relativelocation_x _relativelocation_y _relativelocation_z) (`KismetMathLibrary.BreakVector` (`SceneComponent.RelativeLocation` UFO)))
  (return (`KismetMathLibrary.MakeVector` (+ _relativelocation_x (`self.MoveDistance`)) _relativelocation_y _relativelocation_z) (`SceneComponent.RelativeRotation` UFO)))

(fn `MoveForward`
  (params (UFO :type "SceneComponent Object Reference"))
  (returns (NewPosition :type "Vector Structure") (NewRotation :type "Rotator Structure"))
  (bind (_relativelocation_x _relativelocation_y _relativelocation_z) (`KismetMathLibrary.BreakVector` (`SceneComponent.RelativeLocation` UFO)))
  (return (`KismetMathLibrary.MakeVector` (- _relativelocation_x (`self.MoveDistance`)) _relativelocation_y _relativelocation_z) (`SceneComponent.RelativeRotation` UFO)))

(fn `StopForSeconds`
  (params (StopTime :type Integer :default 10))
  (set `/Game/GameMode/BP_GameMode.Deceleration` true (`self.MyGameMode`)))

(fn `UserConstructionScript`)