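; BP_Bonus_Passing is a bonus pickup that lets the player pass through walls.
; On BeginPlay it calls the parent and sets ActivatedTime to 10.
; When the player character overlaps it, it prints a debug message, calls ActivatePassThroughWalls on MyGameMode and destroys itself.
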(event `self.ReceiveBeginPlay`
  (`parent.ReceiveBeginPlay`)
  ;[1 1 1] Add due to level
  (set `self.ActivatedTime` 10))

(event `self.ReceiveActorBeginOverlap`
  (params (OtherActor :type "Actor Object Reference"))
  (if (== (`GameplayStatics.GetPlayerCharacter` 0) OtherActor)
    (`KismetSystemLibrary.PrintString` "passing activated")
    (`/Game/GameMode/BP_GameMode.ActivatePassThroughWalls` (`self.MyGameMode`))
    (`self.K2_DestroyActor`)))

(fn `UserConstructionScript`
  (`parent.UserConstructionScript`))