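; Game mode that starts a game session and holds flags for pass-through-wall and deceleration effects.
; On BeginPlay, StartGame copies the level from BP_Game_Instance, spawns and stores a BP_Bonus at the game mode's X/Y with a fixed height, and clears Reload.
; Two activation functions only set their effect flags; nothing here applies or resets them.
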(event `self.ReceiveBeginPlay`
  (`self.StartGame`))

(fn `ActivateDeceleration`
  (set `self.Deceleration` true))

(fn `ActivatePassThroughWalls`
  (set `self.PassWalls` true)
  (`KismetSystemLibrary.PrintString` "pass walls"))

(fn `UserConstructionScript`)